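; BP_LightPuzzle is a laser puzzle actor that clears itself once its beam hits the target.
; BeginPlay spawns the lightboard mesh and target at marker components, moves the child-actor laser to BeamSpawn and activates it unless Disabled.
; Tick polls the beam's HitTarget; on a match it deactivates the beam, waits briefly, then destroys itself and both spawned actors.
; A random-selection branch in BeginPlay is unreachable and empty.
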(event EventBeginPlay
  (bind _returnvalue (Math|Random|RandomInteger 3))
  (bind _childactor (Variables|Default|GetChildActor))
  (if (== 1 1)
    (bind _returnvalue_2 (Game|SpawnActorfromClass "/Game/Joe/BP_Lightboard1Mesh.BP_Lightboard1Mesh_C" (Transformation|GetWorldTransform (Variables|Default|GetBase)) "Undefined" "MultiplyWithRoot" 0 0))
    (bind _returnvalue_3 (Game|SpawnActorfromClass "/Game/Joe/SimpleLasers/LaserControls/Target.Target_C" (Transformation|GetWorldTransform (Variables|Default|GetTarget1)) "Undefined" "MultiplyWithRoot" 0 0))
    (Transformation|SetWorldTransform _childactor (Transformation|GetWorldTransform (Variables|Default|GetBeamSpawn)) false false)
    (if (not (Variables|Default|GetDisabled))
      (bind _asbp_laser_beam (Utilities|Casting|CastToBP_LaserBeam (Variables|/Script/Engine.ChildActorComponent|GetChildActor _childactor)))
      (bind _output_get (Variables|Default|SetAs%20BP%20Laser%20Beam _asbp_laser_beam))
      (Default|Activate _output_get))
    (elif (not (== _returnvalue 2))
      (if (== _returnvalue 3)
        _))))

(event EventTick
  (params (DeltaSeconds :type Float%20%28single-precision%29))
  (if (== (Variables|/Game/Joe/SimpleLasers/BP_LaserBeam.BP_LaserBeam_C|GetHitTarget (stale EventBeginPlay _output_get)) (stale EventBeginPlay _returnvalue_3))
    (Default|Deactivate (stale EventBeginPlay _output_get))
    (Utilities|FlowControl|Delay 1.0)
    (Actor|DestroyActor)
    (Actor|DestroyActor (stale EventBeginPlay _returnvalue_3))
    (Actor|DestroyActor (stale EventBeginPlay _returnvalue_2))))

(fn ConstructionScript)