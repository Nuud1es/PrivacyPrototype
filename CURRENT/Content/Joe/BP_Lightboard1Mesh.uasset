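; BP_Lightboard1Mesh is a light board Blueprint that picks one of three board meshes at random when play begins.
; BeginPlay sets BoardMesh to LightBoard1, LightBoard2 or LightBoard3 through two nested random-integer checks.
; Each check makes its own roll, so the odds are uneven and favor LightBoard3.
; The construction script is empty, so the random choice happens only at runtime.
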(event EventBeginPlay
  (bind _returnvalue (Math|Random|RandomInteger 3))
  ;[0.15 0.1207 0 0.5] Spawn 1 of 3 options of board mesh
  (if (== _returnvalue 1)
    (Components|StaticMesh|SetStaticMesh (Variables|Default|GetBoardMesh) "/Game/Joe/LightBoard1.LightBoard1")
    (elif (== _returnvalue 2)
      (Components|StaticMesh|SetStaticMesh (Variables|Default|GetBoardMesh) "/Game/Joe/LightBoard2.LightBoard2")
      (else
        (Components|StaticMesh|SetStaticMesh (Variables|Default|GetBoardMesh) "/Game/Joe/LightBoard3.LightBoard3")))))

(fn ConstructionScript)