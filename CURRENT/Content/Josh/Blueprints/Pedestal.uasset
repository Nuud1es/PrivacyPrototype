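; Pedestal actor that displays an anchor hologram, lifting it clear of the pedestal so the whole object is visible.
; On BeginPlay it spawns a BP_TestAnchor at its Spawnpoint with the Cone as test hologram and keeps a reference.
; When that hologram begins overlapping the Cube, Tick and a Gate switch on, nudging it up each frame until the overlap ends, then both switch off.
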(event OnComponentBeginOverlap(Cube)
  (params (OverlappedComponent :type Primitive%20Component%20Object%20Reference) (OtherActor :type Actor%20Object%20Reference) (OtherComp :type Primitive%20Component%20Object%20Reference) (OtherBodyIndex :type Integer) (bFromSweep :type Boolean) (SweepResult :type Hit%20Result%20Structure%20%28by%20ref%29))
  (bind _anchorref (Variables|Default|GetAnchorRef))
  (bind _hologram (Variables|/Game/Josh/Blueprints/TestingBPs/BP_TestAnchor.BP_TestAnchor_C|GetHologram _anchorref))
  (if (== OtherComp (Variables|/Game/Josh/Blueprints/TestingBPs/BP_TestAnchor.BP_TestAnchor_C|GetHologram (Variables|Default|GetAnchorRef)))
    (Actor|Tick|SetActorTickEnabled true)
    ;[0 0.3158 0.651 0.5] When the hologram overlaps the pedestal itself, move it up so the whole object is shown.
    (Utilities|FlowControl|Gate true) ; enters at Open
  ))

(event EventBeginPlay
  ;[0 0 0 0.5] Should just place an anchor and bpi it but eh
  (bind _returnvalue (Game|SpawnActorfromClass "/Game/Josh/Blueprints/TestingBPs/BP_TestAnchor.BP_TestAnchor_C" (Transformation|GetWorldTransform (Variables|Default|GetSpawnpoint)) "Undefined" "MultiplyWithRoot" self "/Engine/BasicShapes/Cone.Cone" 0.2 0))
  (Variables|Default|SetAnchorRef _returnvalue))

(event EventTick
  (params (DeltaSeconds :type Float%20%28single-precision%29))
  (bind _anchorref (Variables|Default|GetAnchorRef))
  (bind _hologram (Variables|/Game/Josh/Blueprints/TestingBPs/BP_TestAnchor.BP_TestAnchor_C|GetHologram _anchorref))
  ;[0 0.3158 0.651 0.5] When the hologram overlaps the pedestal itself, move it up so the whole object is shown.
  (Utilities|FlowControl|Gate true :!label _label
    (:Exit
      (Transformation|AddLocalOffset _hologram "0.000000,0.000000,5.000000" false false)
      (if (not (Class|PrimitiveComponent|IsOverlappingComponent (Variables|Default|GetCube) _hologram))
        (Actor|Tick|SetActorTickEnabled false)
        (goto _label Close)))))

(fn ConstructionScript)