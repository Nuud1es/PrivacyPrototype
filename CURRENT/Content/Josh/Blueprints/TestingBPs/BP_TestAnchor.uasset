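; Test anchor actor that previews where an attachable object would go using a hologram mesh.
; Its Detection volume notifies BPI_Attachable actors when they begin overlapping and when the tracked one leaves.
; GiveMesh copies mesh and scale onto the hologram, then nudges it downward until it overlaps the owner.
; Attaching records the actor, hides the hologram and disables detection overlaps; detaching restores them.
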(event OnComponentBeginOverlap(Detection)
  (params (OverlappedComponent :type Primitive%20Component%20Object%20Reference) (OtherActor :type Actor%20Object%20Reference) (OtherComp :type Primitive%20Component%20Object%20Reference) (OtherBodyIndex :type Integer) (bFromSweep :type Boolean) (SweepResult :type Hit%20Result%20Structure%20%28by%20ref%29))
  (if (Utilities|DoesObjectImplementInterface OtherActor "/Game/Josh/Blueprints/BPI_Attachable.BPI_Attachable_C")
    (Class|BPIAttachable|OverlappingAnchor(Message) OtherActor self)
    (Variables|Default|SetOverlappedActor OtherActor)))

(event OnComponentEndOverlap(Detection)
  (params (OverlappedComponent :type Primitive%20Component%20Object%20Reference) (OtherActor :type Actor%20Object%20Reference) (OtherComp :type Primitive%20Component%20Object%20Reference) (OtherBodyIndex :type Integer))
  (bind _overlappedactor (Variables|Default|GetOverlappedActor))
  (if (== OtherActor _overlappedactor)
    (Rendering|SetVisibility (Variables|Default|GetHologram) false false)
    (Class|BPIAttachable|LostAnchor(Message) _overlappedactor)))

(event Custom|GiveMesh
  (params (Mesh%20Data :type S%20Mesh%20Data%20Structure))
  (bind _hologram (Variables|Default|GetHologram))
  ;[0 0 0] Gets mesh data including relative component scale so the hologram looks the same as the object to attach
  (Components|StaticMesh|SetStaticMesh _hologram (.mesh Mesh%20Data))
  (Transformation|SetRelativeScale3D _hologram (.localscale Mesh%20Data))
  (Rendering|Material|SetMaterial _hologram 0 "/Game/Josh/Materials/M_ItemHologram.M_ItemHologram")
  (Rendering|SetVisibility _hologram true false)
  (if (not (Collision|IsOverlappingActor (Variables|Default|GetHologram) (Components|GetOwner) :!class /Script/Engine.PrimitiveComponent)) :!label _label
    (Transformation|AddLocalOffset (Variables|Default|GetHologram) "0.000000,0.000000,-5.000000" false false)
    (goto _label)))

(event EventBeginPlay
  (Rendering|SetVisibility (Variables|Default|GetHologram) false false))

(event EventAttachtoAnchor
  (Rendering|SetVisibility (Variables|Default|GetHologram) false false)
  (Variables|/Script/Engine.PrimitiveComponent|SetbGenerateOverlapEvents (Variables|Default|GetDetection) false)
  (Variables|Default|SetAttachedActor (Variables|Default|GetOverlappedActor)))

(event EventDetachfromAnchor
  (Variables|/Script/Engine.PrimitiveComponent|SetbGenerateOverlapEvents (Variables|Default|GetDetection) true)
  (Utilities|IsValid (Variables|Default|GetOverlappedActor)
    (:Is%20Valid
      (Rendering|SetVisibility (Variables|Default|GetHologram) true false))))

(fn ConstructionScript
  (bind _hologram (Variables|Default|GetHologram))
  (Components|StaticMesh|SetStaticMesh _hologram (Variables|Default|GetTestHolo))
  (Transformation|SetWorldScale3D _hologram (Math|Conversions|ToVector(Float) (Variables|Default|GetConstructScale)))
  (Rendering|Material|SetMaterial _hologram 0 "/Game/Josh/Materials/M_ItemHologram.M_ItemHologram"))