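; BP_TestPlayer is a test player Blueprint for exercising the dish minigame.
; On BeginPlay it shows the mouse cursor and enables click events on the player controller.
; Keys 1 and 2 move the actor to hard-coded locations, then reset or begin the game on DishMinigameRef, respectively.
; A Winstate event only prints a win message.
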(event EventBeginPlay
  (bind _returnvalue (Game|GetPlayerController 0))
  (Variables|/Script/Engine.PlayerController|SetbShowMouseCursor _returnvalue true)
  (Variables|/Script/Engine.PlayerController|SetbEnableClickEvents _returnvalue true))

(event EventWinstate
  (params (NewParam :type Boolean))
  (Development|PrintString "Win"))

(event Input|KeyboardEvents|2
  (params (Key :type Key%20Structure))
  (:Pressed
    (Transformation|SetActorLocation "340.000000,1450.000000,300.000000" false false)
    (CallFunction|BeginGame (.DishMinigameRef (Variables|Default|GetDishMinigameRef)))))

(event Input|KeyboardEvents|1
  (params (Key :type Key%20Structure))
  (:Pressed
    (Transformation|SetActorLocation "70.000000,-210.000000,300.000000" false false)
    (CallFunction|ResetGame (.DishMinigameRef (Variables|Default|GetDishMinigameRef)))))

(fn ConstructionScript)