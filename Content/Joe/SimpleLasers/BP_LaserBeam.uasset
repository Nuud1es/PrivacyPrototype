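; BP_LaserBeam is a laser that draws its path from stretched mesh segments, bouncing off mirrors and passing through glass or hidden actors.
; Activate opens a gate into a capped DoN loop that line-traces each segment, reflecting about hit normals or ignoring see-through actors.
; A blocking hit spawns brief sparks and calls LaserStrike, which switches to the alarm material for the player pawn.
; Segments are destroyed after RedrawDelay, and UpdateType controls automatic redraws.
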(event Custom|Activate
  (bind _beamwidth (Variables|Default|GetBeamWidth))
  (bind _beamwidth_2 (Variables|Default|GetBeamWidth))
  ;[1 1 1] Update and draw function
  (Utilities|FlowControl|Sequence
    (:then_0
      (goto _label Open))
    (:then_1
      (Utilities|FlowControl|Gate true :!label _label ; Master control for laser drawing
        (:Exit
          (Variables|Default|SetIncomingLocation (Transformation|GetWorldLocation (Variables|Default|Getroot)))
          (Variables|Default|SetIncomingRotation (Transformation|GetActorRotation))
          (Utilities|FlowControl|Sequence
            (:then_0
              (goto _label_2 Reset))
            (:then_1
              (Utilities|FlowControl|DoN 999 :!label _label_2 ; Finite but arbitrarily large constraint against infinite loops
                (:Exit
                  (bind _returnvalue (AddComponent|AddStaticMeshComponent false))
                  (Utilities|FlowControl|Sequence
                    (:then_0
                      (Variables|/Script/Engine.ActorComponent|SetComponentTags _returnvalue (Utilities|Array|MakeArray "BeamSegment"))
                      (Collision|SetCollisionEnabled _returnvalue "NoCollision")
                      (Components|StaticMesh|SetStaticMesh _returnvalue "/Game/Joe/SimpleLasers/Meshes/SM_LaserBeam.SM_LaserBeam")
                      (Rendering|Material|SetMaterial _returnvalue 0 (Variables|Default|GetBeamMaterial))
                      (Variables|Default|SetCurrentCylinder _returnvalue)
                      (Transformation|SetWorldLocationAndRotation (Variables|Default|GetCurrentCylinder) (Variables|Default|GetIncomingLocation) (Variables|Default|GetIncomingRotation) false false)
                      ;;[1 1 1] Virtually draw one beam segment, gathering data for constructing a static mesh
                      (Utilities|Array|Add (Variables|Default|GetCylinderSet) (Variables|Default|GetCurrentCylinder))
                      (bind _outhit (Collision|LineTraceByChannel (+ (Variables|Default|GetIncomingLocation) (Math|Vector|RotateVector "1.000000, 0, 0" (Variables|Default|GetIncomingRotation))) (+ (+ (Variables|Default|GetIncomingLocation) (Math|Vector|RotateVector "1.000000, 0, 0" (Variables|Default|GetIncomingRotation))) (Math|Vector|RotateVector "100000.000000, 0, 0" (Variables|Default|GetIncomingRotation))) "TraceTypeQuery2" false (Variables|Default|GetActorsToIgnore) "None"))
                      (Variables|Default|SetHitTarget (.hitactor _outhit))
                      (if (.bblockinghit _outhit)
                        ;;[1 1 1] Mark any invisible or glass actors and reiterate, drawing through them
                        (if (or (Utilities|Array|ContainsItem (Variables|Default|GetGlassMaterials) (Rendering|Material|GetMaterial (.hitcomponent _outhit) 0)) (Variables|/Script/Engine.Actor|GetbHidden (.hitactor _outhit)))
                          (Utilities|Array|Add (Variables|Default|GetActorsToIgnore) (.hitactor _outhit))
                          (goto _label_2)
                          (else
                            (Transformation|SetWorldScale3D (Variables|Default|GetCurrentCylinder) (Math|Vector|MakeVector (/ (+ (.distance _outhit) 1.0) 1e+02) _beamwidth_2 _beamwidth_2))
                            ;;[1 1 1] Determine whether to reiterate off a reflective surface or stop
                            (if (or (Actor|ActorHasTag (.hitactor _outhit) "mirror") (Utilities|Array|ContainsItem (Variables|Default|GetMirroredMaterials) (Rendering|Material|GetMaterial (.hitcomponent _outhit) 0)))
                              (Variables|Default|SetIncomingLocation (.location _outhit))
                              (Variables|Default|SetIncomingRotation (Math|Rotator|FindLookatRotation (.location _outhit) (+ (Math|Vector|MirrorVectorbyNormal (Math|Vector|RotateVector "8000.000000, 0, 0" (Variables|Default|GetIncomingRotation)) (.normal _outhit)) (.location _outhit))))
                              (goto _label_2)
                              (else
                                ;;[1 1 1] End condition, a blocking surface has been found
                                (bind _returnvalue_2 (Game|SpawnActorfromClass "/Game/Joe/SimpleLasers/DemoContent/StarterContent/Blueprints/Blueprint_Effect_Sparks.Blueprint_Effect_Sparks_C" (Math|Transform|MakeTransform (.location _outhit) "0, 0, 0" "1.000000,1.000000,1.000000") "Undefined" "OverrideRootScale" 0 0))
                                (Actor|SetLifeSpan _returnvalue_2 0.1)
                                (CallFunction|LaserStrike (.hitactor _outhit) (.hitcomponent _outhit) (.location _outhit))))))
                        (else
                          ;;[1 1 1] Condition used if no surface is found, ie firing into thin air
                          (Transformation|SetWorldScale3D (Variables|Default|GetCurrentCylinder) (Math|Vector|MakeVector 1e+03 _beamwidth _beamwidth))))
                      (Utilities|FlowControl|Delay (+ (Variables|Default|GetRedrawDelay) 0.01))
                      (if (Utilities|Enum|Equal(Enum) "NewEnumerator0" (Variables|Default|GetUpdateType))
                        (CallFunction|UpdatePath)))
                    (:then_1
                      (Utilities|FlowControl|Delay (Variables|Default|GetRedrawDelay))
                      (for _array_element (Actor|GetComponentsbyTag "/Script/Engine.StaticMeshComponent" "BeamSegment")
                        (Components|DestroyComponent _array_element)))))))))))))

(event Custom|Deactivate
  (bind _beamwidth (Variables|Default|GetBeamWidth))
  (bind _beamwidth_2 (Variables|Default|GetBeamWidth))
  ;[1 1 1] Update and draw function
  (Utilities|FlowControl|Gate true) ; enters at Close
)

(event Custom|LaserStrike
  (params (StruckActor :type Actor%20Object%20Reference) (Struck%20Component :type Primitive%20Component%20Object%20Reference) (ExactLocation :type Vector))
  ;[1 1 1] Build off behavior for when the laser hits something
  (if (== StruckActor (Game|Player|GetPlayerPawn 0))
    (Variables|Default|SetBeamMaterial "/Game/Joe/SimpleLasers/Materials/M_AlarmBeam.M_AlarmBeam")
    (else
      (Variables|Default|SetBeamMaterial "/Game/Joe/SimpleLasers/Materials/M_Beam.M_Beam"))))

(event Custom|UpdatePath
  (bind _beamwidth (Variables|Default|GetBeamWidth))
  (bind _beamwidth_2 (Variables|Default|GetBeamWidth))
  ;[1 1 1] Update and draw function
  ;;[1 1 1] Reboot and clean the previous path before redrawing
  (for _array_element (Actor|GetComponentsbyTag "/Script/Engine.StaticMeshComponent" "BeamSegment")
    (Components|DestroyComponent _array_element))
  (Utilities|FlowControl|Gate true ; Master control for laser drawing
    (:Exit
      (Variables|Default|SetIncomingLocation (Transformation|GetWorldLocation (Variables|Default|Getroot)))
      (Variables|Default|SetIncomingRotation (Transformation|GetActorRotation))
      (Utilities|FlowControl|Sequence
        (:then_0
          (goto _label Reset))
        (:then_1
          (Utilities|FlowControl|DoN 999 :!label _label ; Finite but arbitrarily large constraint against infinite loops
            (:Exit
              (bind _returnvalue (AddComponent|AddStaticMeshComponent false))
              (Utilities|FlowControl|Sequence
                (:then_0
                  (Variables|/Script/Engine.ActorComponent|SetComponentTags _returnvalue (Utilities|Array|MakeArray "BeamSegment"))
                  (Collision|SetCollisionEnabled _returnvalue "NoCollision")
                  (Components|StaticMesh|SetStaticMesh _returnvalue "/Game/Joe/SimpleLasers/Meshes/SM_LaserBeam.SM_LaserBeam")
                  (Rendering|Material|SetMaterial _returnvalue 0 (Variables|Default|GetBeamMaterial))
                  (Variables|Default|SetCurrentCylinder _returnvalue)
                  (Transformation|SetWorldLocationAndRotation (Variables|Default|GetCurrentCylinder) (Variables|Default|GetIncomingLocation) (Variables|Default|GetIncomingRotation) false false)
                  ;;[1 1 1] Virtually draw one beam segment, gathering data for constructing a static mesh
                  (Utilities|Array|Add (Variables|Default|GetCylinderSet) (Variables|Default|GetCurrentCylinder))
                  (bind _outhit (Collision|LineTraceByChannel (+ (Variables|Default|GetIncomingLocation) (Math|Vector|RotateVector "1.000000, 0, 0" (Variables|Default|GetIncomingRotation))) (+ (+ (Variables|Default|GetIncomingLocation) (Math|Vector|RotateVector "1.000000, 0, 0" (Variables|Default|GetIncomingRotation))) (Math|Vector|RotateVector "100000.000000, 0, 0" (Variables|Default|GetIncomingRotation))) "TraceTypeQuery2" false (Variables|Default|GetActorsToIgnore) "None"))
                  (Variables|Default|SetHitTarget (.hitactor _outhit))
                  (if (.bblockinghit _outhit)
                    ;;[1 1 1] Mark any invisible or glass actors and reiterate, drawing through them
                    (if (or (Utilities|Array|ContainsItem (Variables|Default|GetGlassMaterials) (Rendering|Material|GetMaterial (.hitcomponent _outhit) 0)) (Variables|/Script/Engine.Actor|GetbHidden (.hitactor _outhit)))
                      (Utilities|Array|Add (Variables|Default|GetActorsToIgnore) (.hitactor _outhit))
                      (goto _label)
                      (else
                        (Transformation|SetWorldScale3D (Variables|Default|GetCurrentCylinder) (Math|Vector|MakeVector (/ (+ (.distance _outhit) 1.0) 1e+02) _beamwidth_2 _beamwidth_2))
                        ;;[1 1 1] Determine whether to reiterate off a reflective surface or stop
                        (if (or (Actor|ActorHasTag (.hitactor _outhit) "mirror") (Utilities|Array|ContainsItem (Variables|Default|GetMirroredMaterials) (Rendering|Material|GetMaterial (.hitcomponent _outhit) 0)))
                          (Variables|Default|SetIncomingLocation (.location _outhit))
                          (Variables|Default|SetIncomingRotation (Math|Rotator|FindLookatRotation (.location _outhit) (+ (Math|Vector|MirrorVectorbyNormal (Math|Vector|RotateVector "8000.000000, 0, 0" (Variables|Default|GetIncomingRotation)) (.normal _outhit)) (.location _outhit))))
                          (goto _label)
                          (else
                            ;;[1 1 1] End condition, a blocking surface has been found
                            (bind _returnvalue_2 (Game|SpawnActorfromClass "/Game/Joe/SimpleLasers/DemoContent/StarterContent/Blueprints/Blueprint_Effect_Sparks.Blueprint_Effect_Sparks_C" (Math|Transform|MakeTransform (.location _outhit) "0, 0, 0" "1.000000,1.000000,1.000000") "Undefined" "OverrideRootScale" 0 0))
                            (Actor|SetLifeSpan _returnvalue_2 0.1)
                            (CallFunction|LaserStrike (.hitactor _outhit) (.hitcomponent _outhit) (.location _outhit))))))
                    (else
                      ;;[1 1 1] Condition used if no surface is found, ie firing into thin air
                      (Transformation|SetWorldScale3D (Variables|Default|GetCurrentCylinder) (Math|Vector|MakeVector 1e+03 _beamwidth _beamwidth))))
                  (Utilities|FlowControl|Delay (+ (Variables|Default|GetRedrawDelay) 0.01))
                  (if (Utilities|Enum|Equal(Enum) "NewEnumerator0" (Variables|Default|GetUpdateType))
                    (CallFunction|UpdatePath)))
                (:then_1
                  (Utilities|FlowControl|Delay (Variables|Default|GetRedrawDelay))
                  (for _array_element_2 (Actor|GetComponentsbyTag "/Script/Engine.StaticMeshComponent" "BeamSegment")
                    (Components|DestroyComponent _array_element_2)))))))))))

(event EventBeginPlay
  (bind _actorstoignore (Variables|Default|GetActorsToIgnore))
  ;[1 1 1] Pass in ignored actors
  (Utilities|Array|Add _actorstoignore (Game|GetInstigator))
  (Utilities|Array|Add _actorstoignore (Actor|GetParentActor)))

(fn ConstructionScript)