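; BP_button runs a button puzzle that spawns one ButtonActor at a time at a random XY position within fixed bounds and height.
; Tick polls the button's ButtonState, then destroys it, increments a count and loops back to the BeginPlay spawn.
; At ten presses it sets ButtonPuzzleCompleted and destroys itself after a short delay, though the sequence still spawns another button.
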(event EventBeginPlay
  (bind _returnvalue (Game|SpawnActorfromClass "/Game/Joe/VRE/Grippables/Misc/Examples/Button/ButtonActor.ButtonActor_C" (Math|Transform|MakeTransform (Math|Vector|MakeVector (Math|Random|RandomFloatinRange 0.0 9e+01) (Math|Random|RandomFloatinRange 0.0 1.8e+02) 2.8e+02) "0, 0, 0" "1.000000,1.000000,1.000000") "Undefined" "MultiplyWithRoot" 0 0 0))
  (Variables|Default|Setbutton _returnvalue))

(event Collision|EventActorBeginOverlap
  (params (OtherActor :type Actor%20Object%20Reference)))

(event EventTick
  (params (DeltaSeconds :type Float%20%28single-precision%29))
  (if (Variables|/Script/VRExpansionPlugin.VRButtonComponent|GetbButtonState (Variables|/Game/Joe/VRE/Grippables/Misc/Examples/Button/ButtonActor.ButtonActor_C|GetButtonComp (Variables|Default|Getbutton)))
    (Development|PrintString (Utilities|String|ToString(Boolean) (Variables|Default|GetButtonPuzzleCompleted)))
    (Utilities|FlowControl|Sequence
      (:then_0
        (Actor|DestroyActor (Variables|Default|Getbutton))
        (Utilities|FlowControl|Sequence
          (:then_0
            (Variables|Default|Setbutton%20count (+ (Variables|Default|Getbutton%20count) 1.0))
            (if (== (Variables|Default|Getbutton%20count) 1e+01)
              (Variables|Default|SetButtonPuzzleCompleted true)
              (Utilities|FlowControl|Delay 0.2)
              (Actor|DestroyActor)))))
      (:then_1
        (bind _returnvalue (Game|SpawnActorfromClass "/Game/Joe/VRE/Grippables/Misc/Examples/Button/ButtonActor.ButtonActor_C" (Math|Transform|MakeTransform (Math|Vector|MakeVector (Math|Random|RandomFloatinRange 0.0 9e+01) (Math|Random|RandomFloatinRange 0.0 1.8e+02) 2.8e+02) "0, 0, 0" "1.000000,1.000000,1.000000") "Undefined" "MultiplyWithRoot" 0 0 0))
        (Variables|Default|Setbutton _returnvalue)))))

(fn ConstructionScript)