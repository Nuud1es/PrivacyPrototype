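; VR dial puzzle actor that spawns three SnapDials at placed points and passes a material along In, Mid and Out pieces.
; Each Tick copies material down the chain, resetting pieces whose dial (first or second) points Up, Down or Left; SetMaterial ignores its Direction input.
; A green Out only prints "completed".
; The third dial affects no named piece, and procedural randomisation is disconnected.
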(event EventTick
  (params (DeltaSeconds :type Float%20%28single-precision%29))
  (bind _out (Variables|Default|Getout))
  (bind _dialref2 (Variables|Default|GetDialRef2))
  (bind _dialref3 (Variables|Default|GetDialRef3))
  (bind _dialref1 (Variables|Default|GetDialRef1))
  (bind _mid (Variables|Default|Getmid))
  (Utilities|FlowControl|Sequence
    (:then_0
      (bind (_up _down _left _right) (Default|GetAngle _dialref1 (Variables|/Script/VRExpansionPlugin.VRDialComponent|GetCurrentDialAngle (Variables|/Game/Joe/SnapDial.SnapDial_C|GetVRDial _dialref1))))
      (Utilities|FlowControl|Sequence
        (:then_0
          (CallFunction|SetMaterial (Variables|Default|GetIn) _mid _right))
        (:then_1
          (if (Math|Boolean|ORBoolean _up _down _left)
            (Rendering|Material|SetMaterial _mid 0 "/Game/Joe/VRE/Grippables/Weapons/Misc/Slicer/01_-_Default.01_-_Default")))))
    (:then_1
      (bind (_up_2 _down_2 _left_2 _right_2) (Default|GetAngle _dialref2 (Variables|/Script/VRExpansionPlugin.VRDialComponent|GetCurrentDialAngle (Variables|/Game/Joe/SnapDial.SnapDial_C|GetVRDial _dialref2))))
      (Utilities|FlowControl|Sequence
        (:then_0
          (CallFunction|SetMaterial (Variables|Default|Getmid) _out _right_2))
        (:then_1
          (if (Math|Boolean|ORBoolean _up_2 _down_2 _left_2)
            (Rendering|Material|SetMaterial _out 0 "/Game/Joe/VRE/Grippables/Weapons/Misc/Slicer/01_-_Default.01_-_Default")))))
    (:then_2
      (bind (_up_3 _down_3 _left_3 _right_3) (Default|GetAngle _dialref3 (Variables|/Script/VRExpansionPlugin.VRDialComponent|GetCurrentDialAngle (Variables|/Game/Joe/SnapDial.SnapDial_C|GetVRDial _dialref3))))
      (Utilities|FlowControl|Sequence
        (:then_0
          (CallFunction|SetMaterial 0 0 _down_3))
        (:then_1
          (if (Math|Boolean|ORBoolean _up_3 _left_3 _right_3)
            _))))
    (:then_3
      (if (== (Rendering|Material|GetMaterial (Variables|Default|Getout) 0) "/Game/Joe/jigsaw/Models/Placeholder/GREEN.GREEN")
        (Development|PrintString "completed")))))

(event EventBeginPlay
  (bind _dialpoint1 (Variables|Default|GetDialPoint1))
  (bind _dialpoint2 (Variables|Default|GetDialPoint2))
  (bind _dialpoint3 (Variables|Default|GetDialPoint3))
  (bind _returnvalue (Transformation|GetWorldTransform _dialpoint3))
  (bind _returnvalue_2 (Transformation|GetWorldTransform _dialpoint1))
  (bind _returnvalue_3 (Transformation|GetWorldTransform _dialpoint2))
  (Utilities|FlowControl|Sequence
    (:then_0
      (bind _returnvalue_4 (Game|SpawnActorfromClass "/Game/Joe/SnapDial.SnapDial_C" (Math|Transform|MakeTransform (.location _returnvalue_2) (.rotation _returnvalue_2) "1.000000,1.000000,1.000000") "Undefined" "SelectDefaultAtRuntime" 0 0))
      (Variables|Default|SetDialRef1 _returnvalue_4))
    (:then_1
      (bind _returnvalue_5 (Game|SpawnActorfromClass "/Game/Joe/SnapDial.SnapDial_C" (Math|Transform|MakeTransform (.location _returnvalue_3) (.rotation _returnvalue_3) "1.000000,1.000000,1.000000") "Undefined" "SelectDefaultAtRuntime" 0 0))
      (Variables|Default|SetDialRef2 _returnvalue_5))
    (:then_2
      (bind _returnvalue_6 (Game|SpawnActorfromClass "/Game/Joe/SnapDial.SnapDial_C" (Math|Transform|MakeTransform (.location _returnvalue) (.rotation _returnvalue) "1.000000,1.000000,1.000000") "Undefined" "SelectDefaultAtRuntime" 0 0))
      (Variables|Default|SetDialRef3 _returnvalue_6))))

(fn ConstructionScript)

(fn SetMaterial
  (params (In :type Static%20Mesh%20Component%20Object%20Reference) (Out :type Static%20Mesh%20Component%20Object%20Reference) (Direction :type Boolean))
  (if true
    (Rendering|Material|SetMaterial Out 0 (Rendering|Material|GetMaterial In 0))
    (else
      (Rendering|Material|SetMaterial Out 0 0))))