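; AttachComponent is an overlap-driven attach point that snaps a released BP_Mirror onto itself.
; On overlap, it stores one held mirror as GrabActor, provided IgnoreController is valid and differs from that mirror's MotionController.
; Tick attaches the stored mirror with snapped location and rotation, keeping world scale, whenever its MotionController is invalid.
; Ending overlap with that mirror clears the reference.
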(event Custom|BeginOverlap
  (params (OverlappedComponent :type Primitive%20Component%20Object%20Reference) (OtherActor :type Actor%20Object%20Reference) (OtherComp :type Primitive%20Component%20Object%20Reference) (OtherBodyIndex :type Integer) (bFromSweep :type Boolean) (SweepResult :type Hit%20Result%20Structure%20%28by%20ref%29))
  (bind _ignorecontroller (Variables|Default|GetIgnoreController))
  (Utilities|IsValid (Variables|Default|GetGrabActor)
    (:Is%20Not%20Valid
      (bind _asbp_mirror (Utilities|Casting|CastToBP_Mirror OtherActor))
      (Utilities|IsValid (Variables|/Game/Joe/Blueprints/AttachPoint/BP_Mirror.BP_Mirror_C|GetMotion%20Controller _asbp_mirror)
        (:Is%20Valid
          (Utilities|IsValid _ignorecontroller
            (:Is%20Valid
              (if (!= _ignorecontroller (Variables|/Game/Joe/Blueprints/AttachPoint/BP_Mirror.BP_Mirror_C|GetMotion%20Controller _asbp_mirror))
                (Variables|Default|SetGrabActor _asbp_mirror)))))))))

(event Custom|EndOverlap
  (params (OverlappedComponent :type Primitive%20Component%20Object%20Reference) (OtherActor :type Actor%20Object%20Reference) (OtherComp :type Primitive%20Component%20Object%20Reference) (OtherBodyIndex :type Integer))
  (if (== (Variables|Default|GetGrabActor) OtherActor)
    (Variables|Default|SetGrabActor 0)))

(event EventBeginPlay
  (Collision|BindEventtoOnComponentBeginOverlap (delegate Custom|BeginOverlap))
  (Collision|BindEventtoOnComponentEndOverlap (delegate Custom|EndOverlap)))

(event EventTick
  (params (DeltaSeconds :type Float%20%28single-precision%29))
  (bind _grabactor (Variables|Default|GetGrabActor))
  (Utilities|IsValid _grabactor
    (:Is%20Valid
      (Utilities|IsValid (Variables|/Game/Joe/Blueprints/AttachPoint/BP_Mirror.BP_Mirror_C|GetMotion%20Controller _grabactor)
        (:Is%20Not%20Valid
          (Transformation|AttachComponentToComponent _grabactor self "None" "SnapToTarget" "SnapToTarget" "KeepWorld" true))))))