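; Jigsaw puzzle platform that spawns green, red and pink pieces at a spawn point, staggered by delays after BeginPlay.
; Each colored slot component sets a flag on any overlap, without checking what entered.
; Tick disables physics on each flagged piece and pins it to its slot's transform every frame, setting Completed once all three flags are true.
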(event OnComponentBeginOverlap(Pink)
  (params (OverlappedComponent :type Primitive%20Component%20Object%20Reference) (OtherActor :type Actor%20Object%20Reference) (OtherComp :type Primitive%20Component%20Object%20Reference) (OtherBodyIndex :type Integer) (bFromSweep :type Boolean) (SweepResult :type Hit%20Result%20Structure%20%28by%20ref%29))
  (Variables|Default|SetPinkOverlap? true))

(event OnComponentBeginOverlap(Red)
  (params (OverlappedComponent :type Primitive%20Component%20Object%20Reference) (OtherActor :type Actor%20Object%20Reference) (OtherComp :type Primitive%20Component%20Object%20Reference) (OtherBodyIndex :type Integer) (bFromSweep :type Boolean) (SweepResult :type Hit%20Result%20Structure%20%28by%20ref%29))
  (Variables|Default|SetRedOverlap? true))

(event OnComponentBeginOverlap(Green)
  (params (OverlappedComponent :type Primitive%20Component%20Object%20Reference) (OtherActor :type Actor%20Object%20Reference) (OtherComp :type Primitive%20Component%20Object%20Reference) (OtherBodyIndex :type Integer) (bFromSweep :type Boolean) (SweepResult :type Hit%20Result%20Structure%20%28by%20ref%29))
  (Variables|Default|SetGreenOverlap? true))

(event EventBeginPlay
  (Utilities|FlowControl|Sequence
    (:then_0
      (bind _returnvalue (Game|SpawnActorfromClass "/Game/Joe/jigsaw/Green.Green_C" (Math|Transform|MakeTransform (Transformation|GetWorldLocation (Variables|Default|Getspawn)) "0, 0, 0" "1.000000,1.000000,1.000000") "Undefined" "SelectDefaultAtRuntime" 0 0))
      (Variables|Default|SetGreenRef _returnvalue))
    (:then_1
      (Utilities|FlowControl|Delay 1.0)
      (bind _returnvalue_2 (Game|SpawnActorfromClass "/Game/Joe/jigsaw/Red.Red_C" (Math|Transform|MakeTransform (Transformation|GetWorldLocation (Variables|Default|Getspawn)) "0, 0, 0" "1.000000,1.000000,1.000000") "Undefined" "SelectDefaultAtRuntime" 0 0))
      (Variables|Default|SetRedRef _returnvalue_2))
    (:then_2
      (Utilities|FlowControl|Delay 2.0)
      (bind _returnvalue_3 (Game|SpawnActorfromClass "/Game/Joe/jigsaw/Pink.Pink_C" (Math|Transform|MakeTransform (Transformation|GetWorldLocation (Variables|Default|Getspawn)) "0, 0, 0" "1.000000,1.000000,1.000000") "Undefined" "SelectDefaultAtRuntime" 0 0))
      (Variables|Default|SetPinkRef _returnvalue_3))
    (:then_3
      (Variables|Default|SetPinkOverlap? false)
      (Variables|Default|SetGreenOverlap? false)
      (Variables|Default|SetRedOverlap? false))))

(event Collision|EventActorBeginOverlap
  (params (OtherActor :type Actor%20Object%20Reference)))

(event EventTick
  (params (DeltaSeconds :type Float%20%28single-precision%29))
  (bind _redref (Variables|Default|GetRedRef))
  (bind _red (Variables|Default|GetRed))
  (bind _pinkref (Variables|Default|GetPinkRef))
  (bind _pink (Variables|Default|GetPink))
  (bind _green (Variables|Default|GetGreen))
  (bind _returnvalue (Transformation|GetWorldTransform _green))
  (bind _returnvalue_2 (Transformation|GetWorldTransform _red))
  (bind _returnvalue_3 (Transformation|GetWorldTransform _pink))
  (Utilities|FlowControl|Sequence
    (:then_0
      (if (Variables|Default|GetGreenOverlap?)
        (Physics|SetSimulatePhysics (Variables|/Script/Engine.StaticMeshActor|GetStaticMeshComponent (Variables|Default|GetGreenRef)) false)
        (Transformation|SetWorldLocationAndRotation (Variables|/Script/Engine.StaticMeshActor|GetStaticMeshComponent (Variables|Default|GetGreenRef)) (.location _returnvalue) (.rotation _returnvalue) false false)))
    (:then_1
      (if (Variables|Default|GetRedOverlap?)
        (Physics|SetSimulatePhysics (Variables|/Script/Engine.StaticMeshActor|GetStaticMeshComponent _redref) false)
        (Transformation|SetWorldLocationAndRotation (Variables|/Script/Engine.StaticMeshActor|GetStaticMeshComponent _redref) (.location _returnvalue_2) (.rotation _returnvalue_2) false false)))
    (:then_2
      (if (Variables|Default|GetPinkOverlap?)
        (Physics|SetSimulatePhysics (Variables|/Script/Engine.StaticMeshActor|GetStaticMeshComponent _pinkref) false)
        (Transformation|SetWorldLocationAndRotation (Variables|/Script/Engine.StaticMeshActor|GetStaticMeshComponent _pinkref) (.location _returnvalue_3) (.rotation _returnvalue_3) false false)))
    (:then_3
      (Variables|Default|SetCompleted (Math|Boolean|ANDBoolean (Variables|Default|GetGreenOverlap?) (Variables|Default|GetRedOverlap?) (Variables|Default|GetPinkOverlap?))))))

(fn ConstructionScript)