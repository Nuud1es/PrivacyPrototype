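; CRT reaction-timing actor that spawns a small BP_Button at its Cube and switches a screen plane to a fight material after a fixed delay.
; Tick polls the button and, while AllowPress is set, takes one press, showing AnimationTimer minus the time since AppearTime on a TextRender.
; The branch that blanks the screen, stamps AppearTime and arms AllowPress is disconnected, so it never runs.
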(event EventBeginPlay
  (bind _returnvalue (Game|SpawnActorfromClass "/Game/Joe/Blueprints/BP_Button.BP_Button_C" (Math|Transform|MakeTransform (Transformation|GetWorldLocation (Variables|Default|GetCube)) "0, 0, 0" "0.100000,0.100000,0.100000") "Undefined" "MultiplyWithRoot" 0 0))
  (Variables|Default|SetButton _returnvalue))

(event EventTick
  (params (DeltaSeconds :type Float%20%28single-precision%29))
  (Utilities|FlowControl|Sequence
    (:then_0
      (Utilities|FlowControl|DoOnce false
        (:Completed
          (Utilities|FlowControl|Delay 6.0)
          (Rendering|Material|SetMaterial (Variables|Default|GetPlane1) 0 "/Game/Joe/Footage/M_Fight.M_Fight"))))
    (:then_1
      (if (Variables|/Game/Joe/Blueprints/BP_Button.BP_Button_C|GetPressed (Variables|Default|GetButton))
        (Variables|Default|SetKey%20Press%20time (Utilities|Time|GetGameTimeinSeconds))
        (if (Variables|Default|GetAllow%20Press)
          (Variables|Default|SetAllow%20Press false)
          (Variables|Default|SetKey%20Press%20time (- (Variables|Default|GetKey%20Press%20time) (Variables|Default|GetAppear%20Time)))
          (Variables|Default|SetRecording%20Time (- (Variables|Default|Getanimation%20Timer) (Variables|Default|GetKey%20Press%20time)))
          (Rendering|Components|TextRender|SetText (Variables|Default|GetTextRender) (Utilities|Text|ToText(Float) (Variables|Default|GetRecording%20Time) "HalfToEven")))))))

(fn ConstructionScript)