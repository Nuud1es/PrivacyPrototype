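; BP_PuzzleSpawn is an unfinished puzzle spawner meant to place a dial, jigsaw or button puzzle at its SpawnPoint.
; Its sequence makes a separate random roll per branch, so several or no spawns could result.
; Nothing triggers that sequence: BeginPlay and the construction script are empty.
; The spawn nodes have no class set, and the puzzle references are set to None rather than the spawned actors.
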(event EventBeginPlay)

(fn ConstructionScript)