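; Test actor (called a sponge in its comments) that is clicked to pick up and drop, and can snap onto anchor actors.
; While held, a gated Tick moves it to the surface hit under the cursor and derives its rotation from the impact normal.
; Anchor overlap events store the candidate and call GiveMesh on it.
; Dropping while ready snaps to that anchor and attaches; clicking when anchored detaches it.
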(event Custom|AttachToMouse
  (bind _returnvalue (Game|GetPlayerController 0))
  (bind _hitresult (Game|Player|GetHitResultUnderCursorbyChannel _returnvalue "TraceTypeQuery3" true))
  (bind (_bblockinghit _binitialoverlap _time _distance _location _impactpoint _normal _impactnormal) (Collision|BreakHitResult _hitresult))
  (bind _returnvalue_2 (Math|Rotator|MakeRotfromZ _impactnormal))
  (Variables|Default|SetIsAttachedToMouse true)
  (Actor|Tick|SetActorTickEnabled true)
  (Utilities|FlowControl|Gate true) ; enters at Open
)

(event Custom|DetachFromMouse
  (bind _returnvalue (Game|GetPlayerController 0))
  (bind _overlappedanchor (Variables|Default|GetOverlappedAnchor))
  (bind _hitresult (Game|Player|GetHitResultUnderCursorbyChannel _returnvalue "TraceTypeQuery3" true))
  (bind (_bblockinghit _binitialoverlap _time _distance _location _impactpoint _normal _impactnormal) (Collision|BreakHitResult _hitresult))
  (bind _returnvalue_2 (Math|Rotator|MakeRotfromZ _impactnormal))
  (Variables|Default|SetIsAttachedToMouse false)
  (Actor|Tick|SetActorTickEnabled false)
  (if (Variables|Default|GetReadyToAnchor)
    (Transformation|SetActorLocation (Transformation|GetActorLocation _overlappedanchor) false false)
    (Default|AttachtoAnchor _overlappedanchor)
    (Variables|Default|SetAnchored true)
    (Utilities|FlowControl|Gate true) ; enters at Close
    (else
      (Utilities|FlowControl|Gate true) ; enters at Close
    )))

(event EventTick
  (params (DeltaSeconds :type Float%20%28single-precision%29))
  (bind _returnvalue (Game|GetPlayerController 0))
  (bind _hitresult (Game|Player|GetHitResultUnderCursorbyChannel _returnvalue "TraceTypeQuery3" true))
  (bind (_bblockinghit _binitialoverlap _time _distance _location _impactpoint _normal _impactnormal) (Collision|BreakHitResult _hitresult))
  (bind _returnvalue_2 (Math|Rotator|MakeRotfromZ _impactnormal))
  (Utilities|FlowControl|Gate true
    (:Exit
      ;[1 1 1] Check what the mouse is hovered over and set the sponge to be on top of it.
      (Transformation|SetActorLocation _impactpoint false false)
      (Transformation|SetActorRotation (Math|Rotator|MakeRotator (.roll _returnvalue_2) 0.0 (.yaw _returnvalue_2))))))

(event MouseInput|EventActorOnClicked
  (params (ButtonPressed :type Key%20Structure :default "None"))
  ;[0.02447 0.03588 0.4271] BPI Stuff
  (if (Variables|Default|GetIsAttachedToMouse)
    (CallFunction|DetachfromMouse)
    (elif (Variables|Default|GetAnchored)
      (Default|DetachfromAnchor (Variables|Default|GetOverlappedAnchor))
      (CallFunction|AttachtoMouse)
      (else
        (CallFunction|AttachtoMouse)))))

(event EventOverlappingAnchor
  (params (TriggeredAnchor :type BP%20Test%20Anchor%20Object%20Reference))
  ;[0.02447 0.03588 0.4271] BPI Stuff
  (bind _output_get (Variables|Default|SetOverlappedAnchor TriggeredAnchor))
  (Default|GiveMesh _output_get)
  (Variables|Default|SetReadyToAnchor true))

(event EventLostAnchor
  ;[0.02447 0.03588 0.4271] BPI Stuff
  (Variables|Default|SetReadyToAnchor false))

(fn ConstructionScript)