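; Test actor for a physics object that can be picked up through a GrabComponent and snapped onto anchor actors.
; While grabbed, an overlapped anchor receives its mesh and scale for a hologram; dropping there snaps actor and mesh to the anchor and disables physics.
; Grabbing again detaches it from the anchor.
; Hard impacts play an impulse-scaled chop sound, and older mouse-based attach code remains from earlier testing.
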(event OnDropped(GrabComponent)
  (bind _overlappedanchor (Variables|Default|GetOverlappedAnchor))
  (bind _returnvalue (Transformation|GetActorLocation _overlappedanchor))
  (bind _returnvalue_2 (Transformation|GetActorRotation _overlappedanchor))
  ;[0.02447 0.03588 0.4271] BPI Stuff | Grabbing and anchoring
  ;;[0 0.3919 0.8281 0.5] Check if an anchor has been overlapped and, if so, teleport this actor and its mesh to the anchor origin
  (if (Variables|Default|GetReadyToAnchor)
    (Transformation|SetActorLocationAndRotation _returnvalue _returnvalue_2)
    (Transformation|SetWorldLocationAndRotation (Variables|Default|GetMesh) _returnvalue _returnvalue_2 false false)
    (Default|AttachtoAnchor _overlappedanchor)
    (Physics|SetSimulatePhysics (Variables|Default|GetMesh) false)
    (Variables|Default|SetAnchored true)
    (Variables|Default|SetGrabbed false)
    (else
      (Variables|Default|SetGrabbed false))))

(event OnGrabbed(GrabComponent)
  ;[0.02447 0.03588 0.4271] BPI Stuff | Grabbing and anchoring
  ;;[0 0.3627 0.625 0.5] Check if this actor is anchored, if so, tell the anchor that it is about to detach
  (if (Variables|Default|GetAnchored)
    (Default|DetachfromAnchor (Variables|Default|GetOverlappedAnchor))
    (Variables|Default|SetGrabbed true)
    (else
      (Variables|Default|SetGrabbed true))))

(event Custom|AttachToMouse
  (bind _returnvalue (Game|GetPlayerController 0))
  (bind _hitresult (Game|Player|GetHitResultUnderCursorbyChannel _returnvalue "TraceTypeQuery3" true))
  (bind (_bblockinghit _binitialoverlap _time _distance _location _impactpoint _normal _impactnormal) (Collision|BreakHitResult _hitresult))
  (bind _returnvalue_2 (Math|Rotator|MakeRotfromZ _impactnormal))
  ;[0.15 0.02266 0.02266 0.5] Old mouse code
  (Variables|Default|SetIsAttachedToMouse true)
  (Actor|Tick|SetActorTickEnabled true)
  (Utilities|FlowControl|Gate true ; enters at Open
    (:Exit
      ;;[1 1 1] Check what the mouse is hovered over and set the sponge to be on top of it.
      (Transformation|SetActorLocation _impactpoint false false)
      (Transformation|SetActorRotation (Math|Rotator|MakeRotator (.roll _returnvalue_2) 0.0 (.yaw _returnvalue_2))))))

(event Custom|DetachFromMouse
  (bind _returnvalue (Game|GetPlayerController 0))
  (bind _overlappedanchor (Variables|Default|GetOverlappedAnchor))
  (bind _hitresult (Game|Player|GetHitResultUnderCursorbyChannel _returnvalue "TraceTypeQuery3" true))
  (bind (_bblockinghit _binitialoverlap _time _distance _location _impactpoint _normal _impactnormal) (Collision|BreakHitResult _hitresult))
  (bind _returnvalue_2 (Math|Rotator|MakeRotfromZ _impactnormal))
  ;[0.15 0.02266 0.02266 0.5] Old mouse code
  (Variables|Default|SetIsAttachedToMouse false)
  (Actor|Tick|SetActorTickEnabled false)
  (if (Variables|Default|GetReadyToAnchor)
    (Transformation|SetActorLocation (Transformation|GetActorLocation _overlappedanchor) false false)
    (Default|AttachtoAnchor _overlappedanchor)
    (Variables|Default|SetAnchored true)
    (Utilities|FlowControl|Gate true :!label _label ; enters at Close
      (:Exit
        _))
    (else
      (goto _label Close)))
  ;;[1 1 1] Check what the mouse is hovered over and set the sponge to be on top of it.
  (Transformation|SetActorLocation _impactpoint false false)
  (Transformation|SetActorRotation (Math|Rotator|MakeRotator (.roll _returnvalue_2) 0.0 (.yaw _returnvalue_2))))

(event Collision|EventHit
  (params (MyComp :type Primitive%20Component%20Object%20Reference) (Other :type Actor%20Object%20Reference) (OtherComp :type Primitive%20Component%20Object%20Reference) (bSelfMoved :type Boolean) (HitLocation :type Vector :default "0, 0, 0") (HitNormal :type Vector :default "0, 0, 0") (NormalImpulse :type Vector :default "0, 0, 0") (Hit :type Hit%20Result%20Structure%20%28by%20ref%29))
  (bind _returnvalue (Math|Vector|VectorLength NormalImpulse))
  ;[0.5363 0.5365 0.1257 0.5] Collision sounds
  (if (> _returnvalue 2e+02)
    (Utilities|FlowControl|DoOnce false :!label _label
      (:Completed
        (Audio|PlaySoundatLocation "/Game/Sounds/Hit/Chop_01.Chop_01" HitLocation "0, 0, 0" (Math|Float|Clamp(Float) (/ _returnvalue 1e+03) 0.0 0.7) 1.0 0.0 0 0 0 0)
        (goto _label Reset)))))

(event EventTick
  (params (DeltaSeconds :type Float%20%28single-precision%29)))

(event MouseInput|EventActorOnClicked
  (params (ButtonPressed :type Key%20Structure :default "None"))
  ;[0.02447 0.03588 0.4271] BPI Stuff | Grabbing and anchoring
  ;;[0.2292 0 0 0.5] Old code for when testing with mouse
  (if (Variables|Default|GetIsAttachedToMouse)
    (CallFunction|DetachfromMouse)
    (elif (Variables|Default|GetAnchored)
      (Default|DetachfromAnchor (Variables|Default|GetOverlappedAnchor))
      (CallFunction|AttachtoMouse)
      (else
        (CallFunction|AttachtoMouse)))))

(event EventOverlappingAnchor
  (params (TriggeredAnchor :type BP%20Test%20Anchor%20Object%20Reference))
  (bind _mesh (Variables|Default|GetMesh))
  ;[0.02447 0.03588 0.4271] BPI Stuff | Grabbing and anchoring
  ;;[0 0.3771 0.7188 0.5] When an anchor is overlapped, the anchor will send itself and this actor will send back mesh data for the hologram
  (if (Variables|Default|GetGrabbed)
    (bind _output_get (Variables|Default|SetOverlappedAnchor TriggeredAnchor))
    (Default|GiveMesh _output_get (Utilities|Struct|MakeS_MeshData (Variables|/Script/Engine.StaticMeshComponent|GetStaticMesh _mesh) (.scale (Transformation|GetRelativeTransform _mesh))))
    (Variables|Default|SetReadyToAnchor true)))

(event EventLostAnchor
  ;[0.02447 0.03588 0.4271] BPI Stuff | Grabbing and anchoring
  ;;[0.15 0.15 0.15 0.5] :(
  (Variables|Default|SetReadyToAnchor false))

(fn ConstructionScript)

(fn GiveMesh
  (params (Mesh :type S%20Mesh%20Data%20Structure))
  (return))