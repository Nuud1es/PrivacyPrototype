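; BP_SpawnerButtons is a VR test actor with two grabbable buttons for spawning and clearing test objects.
; Grabbing the first spawns a BP_TestGrabbable at the Spawnpoint, sets its mesh to a cube and stores it in an array.
; Grabbing the second destroys every stored actor and empties the array.
; A random mesh pick from MeshArray is left unconnected.
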(event OnGrabbed(GrabComponent1)
  (for _array_element (Variables|Default|GetSpawnedActorRef)
    (Actor|DestroyActor _array_element))
  (Utilities|Array|Clear (Variables|Default|GetSpawnedActorRef)))

(event OnGrabbed(GrabComponent)
  (bind _returnvalue (Game|SpawnActorfromClass "/Game/Josh/Blueprints/TestingBPs/BP_TestGrabbable.BP_TestGrabbable_C" (Transformation|GetWorldTransform (Variables|Default|GetSpawnpoint)) "Undefined" "MultiplyWithRoot" 0 0))
  (Utilities|Array|Add (Variables|Default|GetSpawnedActorRef) _returnvalue)
  (Components|StaticMesh|SetStaticMesh (Variables|/Game/Josh/Blueprints/TestingBPs/BP_TestGrabbable.BP_TestGrabbable_C|GetMesh _returnvalue) "/Engine/VREditor/BasicMeshes/SM_Cube_01.SM_Cube_01"))

(fn ConstructionScript)